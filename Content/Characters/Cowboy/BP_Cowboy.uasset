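; Cowboy target character that detects projectile hits and scores them by distance to the nearest body weakpoint.
; On BeginPlay it gathers the box components under the rigged mesh as weakpoints.
; A projectile overlap finds the closest box, destroys the projectile, sets and prints Score as that distance times a multiplier, and counts the hit.
; Per-part overlaps only print debug names; fixed per-part score additions are left unconnected.
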(event `self.ReceiveBeginPlay`
  (for _array_element (`SceneComponent.GetChildrenComponents` (`self.PlayerRigged__2_`) false)
    (bind _asbox_collision (cast `BoxComponent` _array_element))
    (`KismetArrayLibrary.Array_Add` (`self.Collisions`) _asbox_collision)))

(event `self.ReceiveTick`
  (params (DeltaSeconds :type "Float (single-precision)")))

(event `self.PlayerRigged__2_.OnComponentBeginOverlap`
  (params (OverlappedComponent :type "PrimitiveComponent Object Reference") (OtherActor :type "Actor Object Reference") (OtherComp :type "PrimitiveComponent Object Reference") (OtherBodyIndex :type Integer) (bFromSweep :type Boolean) (SweepResult :type "HitResult Structure (by ref)"))
  (bind _asa_projectile (cast `A_Projectile` OtherActor))
  (`self.GetClosestWeakpoint` _asa_projectile)
  (bind _output_get (set `self.Score` (* (`self.CurrentSmallestValue`) 10.0)))
  (`KismetSystemLibrary.PrintString` (`KismetStringLibrary.Conv_DoubleToString` _output_get))
  (set `self.CurrentSmallestValue` 99999999.0)
  (set `self.ClosestCollision` null)
  (`/Engine/EditorBlueprintResources/StandardMacros.IncrementInt` (`self.HitsTaken`)))

(event `self.DickCollision.OnComponentBeginOverlap`
  (params (OverlappedComponent :type "PrimitiveComponent Object Reference") (OtherActor :type "Actor Object Reference") (OtherComp :type "PrimitiveComponent Object Reference") (OtherBodyIndex :type Integer) (bFromSweep :type Boolean) (SweepResult :type "HitResult Structure (by ref)"))
  (`self.PrintHitDebug` OtherActor OverlappedComponent))

(event `self.RightKidneyCollision.OnComponentBeginOverlap`
  (params (OverlappedComponent :type "PrimitiveComponent Object Reference") (OtherActor :type "Actor Object Reference") (OtherComp :type "PrimitiveComponent Object Reference") (OtherBodyIndex :type Integer) (bFromSweep :type Boolean) (SweepResult :type "HitResult Structure (by ref)"))
  (`self.PrintHitDebug` OtherActor OverlappedComponent))

(event `self.LeftKidneyCollision.OnComponentBeginOverlap`
  (params (OverlappedComponent :type "PrimitiveComponent Object Reference") (OtherActor :type "Actor Object Reference") (OtherComp :type "PrimitiveComponent Object Reference") (OtherBodyIndex :type Integer) (bFromSweep :type Boolean) (SweepResult :type "HitResult Structure (by ref)"))
  (`self.PrintHitDebug` OtherActor OverlappedComponent))

(event `self.RightElbowCollision.OnComponentBeginOverlap`
  (params (OverlappedComponent :type "PrimitiveComponent Object Reference") (OtherActor :type "Actor Object Reference") (OtherComp :type "PrimitiveComponent Object Reference") (OtherBodyIndex :type Integer) (bFromSweep :type Boolean) (SweepResult :type "HitResult Structure (by ref)"))
  (`self.PrintHitDebug` OtherActor OverlappedComponent))

(event `self.RightHandCollision.OnComponentBeginOverlap`
  (params (OverlappedComponent :type "PrimitiveComponent Object Reference") (OtherActor :type "Actor Object Reference") (OtherComp :type "PrimitiveComponent Object Reference") (OtherBodyIndex :type Integer) (bFromSweep :type Boolean) (SweepResult :type "HitResult Structure (by ref)"))
  (`self.PrintHitDebug` OtherActor OverlappedComponent))

(event `self.LeftHandCollision.OnComponentBeginOverlap`
  (params (OverlappedComponent :type "PrimitiveComponent Object Reference") (OtherActor :type "Actor Object Reference") (OtherComp :type "PrimitiveComponent Object Reference") (OtherBodyIndex :type Integer) (bFromSweep :type Boolean) (SweepResult :type "HitResult Structure (by ref)"))
  (`self.PrintHitDebug` OtherActor OverlappedComponent))

(event `self.LeftElbowCollision.OnComponentBeginOverlap`
  (params (OverlappedComponent :type "PrimitiveComponent Object Reference") (OtherActor :type "Actor Object Reference") (OtherComp :type "PrimitiveComponent Object Reference") (OtherBodyIndex :type Integer) (bFromSweep :type Boolean) (SweepResult :type "HitResult Structure (by ref)"))
  (`self.PrintHitDebug` OtherActor OverlappedComponent))

(event `self.LeftKneeCollision.OnComponentBeginOverlap`
  (params (OverlappedComponent :type "PrimitiveComponent Object Reference") (OtherActor :type "Actor Object Reference") (OtherComp :type "PrimitiveComponent Object Reference") (OtherBodyIndex :type Integer) (bFromSweep :type Boolean) (SweepResult :type "HitResult Structure (by ref)"))
  (`self.PrintHitDebug` OtherActor OverlappedComponent))

(event `self.RightKneeCollision.OnComponentBeginOverlap`
  (params (OverlappedComponent :type "PrimitiveComponent Object Reference") (OtherActor :type "Actor Object Reference") (OtherComp :type "PrimitiveComponent Object Reference") (OtherBodyIndex :type Integer) (bFromSweep :type Boolean) (SweepResult :type "HitResult Structure (by ref)"))
  (`self.PrintHitDebug` OtherActor OverlappedComponent))

(event `self.HeartCollision.OnComponentBeginOverlap`
  (params (OverlappedComponent :type "PrimitiveComponent Object Reference") (OtherActor :type "Actor Object Reference") (OtherComp :type "PrimitiveComponent Object Reference") (OtherBodyIndex :type Integer) (bFromSweep :type Boolean) (SweepResult :type "HitResult Structure (by ref)"))
  (`self.PrintHitDebug` OtherActor OverlappedComponent))

(event `self.NeckCollision.OnComponentBeginOverlap`
  (params (OverlappedComponent :type "PrimitiveComponent Object Reference") (OtherActor :type "Actor Object Reference") (OtherComp :type "PrimitiveComponent Object Reference") (OtherBodyIndex :type Integer) (bFromSweep :type Boolean) (SweepResult :type "HitResult Structure (by ref)"))
  (`self.PrintHitDebug` OtherActor OverlappedComponent))

(event `self.HeadCollision.OnComponentBeginOverlap`
  (params (OverlappedComponent :type "PrimitiveComponent Object Reference") (OtherActor :type "Actor Object Reference") (OtherComp :type "PrimitiveComponent Object Reference") (OtherBodyIndex :type Integer) (bFromSweep :type Boolean) (SweepResult :type "HitResult Structure (by ref)"))
  (`self.PrintHitDebug` OtherActor OverlappedComponent))

(fn `GetClosestWeakpoint`
  (params (Projectile :type "A_Projectile Object Reference"))
  (returns (ClosestWeakpoint :type "SceneComponent Object Reference"))
  (for _array_element (`self.Collisions`)
    (bind _returnvalue (`KismetMathLibrary.Vector_Distance` (`SceneComponent.K2_GetComponentLocation` _array_element) (`SceneComponent.K2_GetComponentLocation` (`A_Projectile.bulletMesh` Projectile))))
    (if (< _returnvalue (`self.CurrentSmallestValue`))
      (set `self.CurrentSmallestValue` _returnvalue)
      (set `self.ClosestCollision` _array_element)))
  (`KismetSystemLibrary.PrintString` (`KismetSystemLibrary.GetObjectName` (`self.ClosestCollision`)))
  (`self.K2_DestroyActor` Projectile)
  (return (`self.ClosestCollision`)))

(fn `PrintHitDebug`
  (params (Object :type "Object Object Reference") (Object2 :type "Object Object Reference"))
  (cast `A_Projectile` Object)
  (`KismetSystemLibrary.PrintString` (`KismetSystemLibrary.GetDisplayName` Object2))
  (return))

(fn `UserConstructionScript`)